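; Example actor that integrates the Stomt feedback widget and lets the player toggle it with the E key.
; BeginPlay enables input, creates StomtWidgetBP and configures its target, app ID, test REST URL and log and screenshot upload options.
; The hotkey opens or closes the widget based on viewport state, then calls the matching open or close dispatcher.
; Unconnected sample nodes show event binding and label assignment but never run.
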(event `self.ReceiveBeginPlay`
  (bind _returnvalue (`GameplayStatics.GetPlayerController` 0))
  ;[0.15 0.15 0.15] Enable Input for Hotkey
  (`self.EnableInput` _returnvalue)
  ;[0.15 0.15 0.15] Create Stomt Widget
  (bind _returnvalue_2 (`|CreateWidget` "/StomtPlugin/Blueprints/Interface/StomtWidgetBP.StomtWidgetBP_C" _returnvalue))
  (bind _output_get (set `self.StomtWidget` _returnvalue_2))
  (set `/StomtPlugin/Blueprints/Interface/StomtWidgetBP.TargetID` "my-my" _output_get)
  (set `/StomtPlugin/Blueprints/Interface/StomtWidgetBP.AppID` "AKN5M7Ob0MqxKXYdE9i3IhQtF" (`self.StomtWidget`))
  (set `/StomtPlugin/Blueprints/Interface/StomtWidgetBP.RestURL` "https://test.rest.stomt.com" (`self.StomtWidget`))
  (set `/StomtPlugin/Blueprints/Interface/StomtWidgetBP.DisableLogUpload` false (`self.StomtWidget`))
  (set `/StomtPlugin/Blueprints/Interface/StomtWidgetBP.DisableScreenshots` false (`self.StomtWidget`)))

(event `Key|E`
  (params (Key :type "Key Structure"))
  (bind _stomtwidget (`self.StomtWidget`))
  ;[0 0.0479 0.3] Hotkey
  (:`Pressed`
    ;[0.15 0.15 0.15] Toggle Widget ON/OFF Hotkey
    (if (`Widget.IsInViewport` (`self.StomtWidget`))
      (`/StomtPlugin/Blueprints/Interface/StomtWidgetBP.Close` _stomtwidget)
      (`self.OnClose`)
      (else
        (`/StomtPlugin/Blueprints/Interface/StomtWidgetBP.Open` _stomtwidget)
        (`self.OnOpen`)))))

(event `YourEvent`
  ;[0.15 0.15 0.15] Bind Events Example
)

(fn `UserConstructionScript`)